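; BP_FlamePillar is a flame pillar actor whose point light flickers in brightness.
; From BeginPlay, ChoseTL randomly picks one of two flicker timelines, and each calls ChoseTL again when finished, giving an endless, varied loop.
; Each timeline update passes its curve value to SetIntensity, which multiplies it by the Intensity variable and applies it to the PointLight.
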(event `ChoseTL`
  ; 注释
  (switch `int` (`KismetMathLibrary.RandomIntegerInRange` 0 1)
    (:`Default`
      (`self.PlayTimeLine_2` :!label _label))
    (:`0`
      (`self.PlayTimeLine_1`))
    (:`1`
      (goto _label))))

(event `self.ReceiveBeginPlay`
  (`self.ChoseTL`))

(event `PlayTimeLine_1`
  ; 注释
  (bind (_direction `_强度`) (`Timeline|亮度闪烁_1` :!via `PlayFromStart`)
    (:`Update`
      (`self.SetIntensity` `_强度`))
    (:`Finished`
      (`self.ChoseTL` :!label _label_2))))

(event `PlayTimeLine_2`
  ; 注释
  (bind (_direction `_强度`) (`Timeline|亮度闪烁_2` :!via `PlayFromStart`)
    (:`Update`
      (`self.SetIntensity` `_强度`))
    (:`Finished`
      (goto _label_2))))

(fn `SetIntensity`
  (params (A :type "Float (double-precision)"))
  (`LightComponent.SetIntensity` (`self.PointLight`) (* A (`self.Intensity`))))

(fn `UserConstructionScript`)